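; BP_ArrowUp is an arrow actor that moves the player up to the height of a linked down arrow.
; Its box collision shows a cone while something overlaps it and hides it on exit.
; On BeginPlay it binds to BP_Jone's interact event, which triggers GoUp.
; If the player overlaps the actor, GoUp teleports them to the ArrowDownReference Z, offset along X, with zeroed rotation.
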(event OnComponentBeginOverlap(BoxCollision)
  (params (OverlappedComponent :type Primitive%20Component%20Object%20Reference) (OtherActor :type Actor%20Object%20Reference) (OtherComp :type Primitive%20Component%20Object%20Reference) (OtherBodyIndex :type Integer) (bFromSweep :type Boolean) (SweepResult :type Hit%20Result%20Structure%20%28by%20ref%29))
  (Rendering|SetVisibility (Variables|Default|GetCone) true false))

(event OnComponentEndOverlap(BoxCollision)
  (params (OverlappedComponent :type Primitive%20Component%20Object%20Reference) (OtherActor :type Actor%20Object%20Reference) (OtherComp :type Primitive%20Component%20Object%20Reference) (OtherBodyIndex :type Integer))
  (Rendering|SetVisibility (Variables|Default|GetCone) false false))

(event Custom|GoUp
  (bind _returnvalue (Game|GetPlayerCharacter 0))
  (bind _returnvalue_2 (Transformation|GetActorLocation _returnvalue))
  (bind (_x _y) (Math|Vector|BreakVector _returnvalue_2))
  (if (Collision|IsOverlappingActor _returnvalue :!class /Script/Engine.Actor)
    (Transformation|Teleport _returnvalue (Math|Vector|MakeVector (+ _x 2e+02) _y (.Z (Math|Vector|BreakVector (Transformation|GetActorLocation (Variables|Default|GetArrowDownReference))))) "0, 0, 0")))

(event Custom|Interact_01
  (CallFunction|GoUp))

(event EventBeginPlay
  (bind _asbp_jone (Utilities|Casting|CastToBP_Jone (Game|GetPlayerCharacter 0)))
  (Variables|Default|SetPlayerReference _asbp_jone)
  (EventDispatchers|BindEventtoInteract _asbp_jone (delegate Custom|Interact_01)))

(event Collision|EventActorBeginOverlap
  (params (OtherActor :type Actor%20Object%20Reference)))

(event EventTick
  (params (DeltaSeconds :type Float%20%28single-precision%29)))

(fn ConstructionScript)