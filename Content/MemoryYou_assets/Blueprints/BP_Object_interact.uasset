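; BP_Object_interact is a world object the player interacts with to receive an item, optionally in exchange for a required one.
; Its collision box shows a linked question-mark actor, enables input and opens a gate while overlapped, reversing this on exit.
; Interact checks BP_Jone for any required item and removes it, then destroys the object and marker and adds the new item.
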(event OnComponentBeginOverlap(BoxCollision)
  (params (OverlappedComponent :type Primitive%20Component%20Object%20Reference) (OtherActor :type Actor%20Object%20Reference) (OtherComp :type Primitive%20Component%20Object%20Reference) (OtherBodyIndex :type Integer) (bFromSweep :type Boolean) (SweepResult :type Hit%20Result%20Structure%20%28by%20ref%29))
  (Rendering|SetVisibility (Variables|/Script/Engine.Actor|GetRootComponent (Variables|Default|GetQuestionMarkReference)) true true)
  (Input|EnableInput (Game|GetPlayerController 0))
  (Utilities|FlowControl|Gate true) ; enters at Open
)

(event OnComponentEndOverlap(BoxCollision)
  (params (OverlappedComponent :type Primitive%20Component%20Object%20Reference) (OtherActor :type Actor%20Object%20Reference) (OtherComp :type Primitive%20Component%20Object%20Reference) (OtherBodyIndex :type Integer))
  (Rendering|SetVisibility (Variables|/Script/Engine.Actor|GetRootComponent (Variables|Default|GetQuestionMarkReference)) false true)
  (Input|DisableInput (Game|GetPlayerController 0))
  (Utilities|FlowControl|Gate true) ; enters at Close
)

(event EventBeginPlay
  (bind _asbp_jone (Utilities|Casting|CastToBP_Jone (Game|GetPlayerCharacter 0)))
  (Variables|Default|SetMainCharacterReference _asbp_jone))

(event Collision|EventActorBeginOverlap
  (params (OtherActor :type Actor%20Object%20Reference)))

(event EventTick
  (params (DeltaSeconds :type Float%20%28single-precision%29)))

(event Input|ActionEvents|InputActionInteract
  (params (Key :type Key%20Structure :default "None"))
  (:Pressed
    (Utilities|FlowControl|Gate true
      (:Exit
        (if (Utilities|Enum|Equal(Enum) (Variables|Default|GetItemRequired) "")
          (Actor|DestroyActor)
          (Actor|DestroyActor (Variables|Default|GetQuestionMarkReference))
          (Default|AddItem (Variables|Default|GetMainCharacterReference) (Variables|Default|GetItemName) :!label _label)
          (else
            (bind _return (Default|FindItemRequired (Variables|Default|GetMainCharacterReference) (Variables|Default|GetItemRequired)))
            (if _return
              (Actor|DestroyActor)
              (Actor|DestroyActor (Variables|Default|GetQuestionMarkReference))
              (Default|RemoveItem (Variables|Default|GetMainCharacterReference) (Variables|Default|GetItemRequired))
              (goto _label))))))))

(fn ConstructionScript)