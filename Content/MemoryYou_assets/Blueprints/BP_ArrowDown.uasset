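; BP_ArrowDown is a placed down-arrow that teleports the player to a linked ArrowUpReference actor.
; Overlapping its box shows a cone marker, enables input and opens a gate; leaving reverses this.
; While the gate is open, pressing GoDown moves the player to the reference's X and Z, keeping the player's own Y and zeroing rotation.
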(event OnComponentBeginOverlap(BoxCollision)
  (params (OverlappedComponent :type Primitive%20Component%20Object%20Reference) (OtherActor :type Actor%20Object%20Reference) (OtherComp :type Primitive%20Component%20Object%20Reference) (OtherBodyIndex :type Integer) (bFromSweep :type Boolean) (SweepResult :type Hit%20Result%20Structure%20%28by%20ref%29))
  (Rendering|SetVisibility (Variables|Default|GetCone) true false)
  (Input|EnableInput (Game|GetPlayerController 0))
  (Utilities|FlowControl|Gate true) ; enters at Open
)

(event OnComponentEndOverlap(BoxCollision)
  (params (OverlappedComponent :type Primitive%20Component%20Object%20Reference) (OtherActor :type Actor%20Object%20Reference) (OtherComp :type Primitive%20Component%20Object%20Reference) (OtherBodyIndex :type Integer))
  (Rendering|SetVisibility (Variables|Default|GetCone) false false)
  (Input|DisableInput (Game|GetPlayerController 0))
  (Utilities|FlowControl|Gate true) ; enters at Close
)

(event Custom|GoDown
  (bind _returnvalue (Game|GetPlayerCharacter 0))
  (bind _arrowupreference (Variables|Default|GetArrowUpReference))
  (bind _returnvalue_2 (Transformation|GetActorLocation _arrowupreference))
  (bind (_x _y _z) (Math|Vector|BreakVector _returnvalue_2))
  (Transformation|Teleport _returnvalue (Math|Vector|MakeVector _x (.Y (Math|Vector|BreakVector (Transformation|GetActorLocation _returnvalue))) _z) "0, 0, 0"))

(event EventBeginPlay
  (Rendering|SetVisibility (Variables|Default|GetCone) false false))

(event Collision|EventActorBeginOverlap
  (params (OtherActor :type Actor%20Object%20Reference)))

(event EventTick
  (params (DeltaSeconds :type Float%20%28single-precision%29)))

(event Input|ActionEvents|InputActionGoDown
  (params (Key :type Key%20Structure :default "None"))
  (:Pressed
    (Utilities|FlowControl|Gate true
      (:Exit
        (CallFunction|GoDown)))))

(fn ConstructionScript)