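; BP_List is a Level02 interactable that plays data-table dialogue and can give the player an item.
; Its box collision toggles a question mark and input; Interact checks for and removes any required item, then advances the message.
; Each step filters table rows by message number, quest completion and repeat flag, showing up to three lines in HUB_Dialogue.
; When messages run out, a first-time dialogue destroys both actors and adds the item.
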(event OnComponentBeginOverlap(BoxCollision)
  (params (OverlappedComponent :type Primitive%20Component%20Object%20Reference) (OtherActor :type Actor%20Object%20Reference) (OtherComp :type Primitive%20Component%20Object%20Reference) (OtherBodyIndex :type Integer) (bFromSweep :type Boolean) (SweepResult :type Hit%20Result%20Structure%20%28by%20ref%29))
  (Rendering|SetVisibility (Variables|/Script/Engine.Actor|GetRootComponent (Variables|Default|GetQuestionMarkReference)) true true)
  (Input|EnableInput (Game|GetPlayerController 0)))

(event OnComponentEndOverlap(BoxCollision)
  (params (OverlappedComponent :type Primitive%20Component%20Object%20Reference) (OtherActor :type Actor%20Object%20Reference) (OtherComp :type Primitive%20Component%20Object%20Reference) (OtherBodyIndex :type Integer))
  (Rendering|SetVisibility (Variables|/Script/Engine.Actor|GetRootComponent (Variables|Default|GetQuestionMarkReference)) false true)
  (Input|DisableInput (Game|GetPlayerController 0))
  (Utilities|IsValid (Variables|Default|GetDialogueWidget)
    (:Is%20Valid
      (Widget|RemovefromParent (Variables|Default|GetDialogueWidget))
      (Variables|Default|SetDialogueWidget 0)
      (Variables|Default|SetMessageCurrent 0))))

(event EventBeginPlay
  (bind _asbp_jone (Utilities|Casting|CastToBP_Jone (Game|GetPlayerCharacter 0)))
  (Variables|Default|SetMainCharacterReference _asbp_jone)
  (bind _outrownames (DataTable|GetDataTableRowNames (Variables|Default|GetDialogueTable)))
  (for _array_element _outrownames
    (Utilities|Array|Add (Variables|Default|GetMyDialogue) _array_element)))

(event Collision|EventActorBeginOverlap
  (params (OtherActor :type Actor%20Object%20Reference)))

(event EventTick
  (params (DeltaSeconds :type Float%20%28single-precision%29)))

(event Input|ActionEvents|InputActionInteract
  (params (Key :type Key%20Structure :default "None"))
  (:Pressed
    (Audio|PlaySound2D "/Game/MemoryYou_assets/Sounds/click.click" 1.0 1.0 0.0 0 0)
    (if (Utilities|Enum|Equal(Enum) (Variables|Default|GetItemRequired) "")
      (Variables|Default|SetQuestionComplete false)
      (Variables|Default|SetAgain false)
      (else
        (bind _return (Default|FindItemRequired (Variables|Default|GetMainCharacterReference) (Variables|Default|GetItemRequired)))
        (if _return
          (Variables|Default|SetQuestionComplete true)
          (Variables|Default|SetAgain false)
          (Default|RemoveItem (Variables|Default|GetMainCharacterReference) (Variables|Default|GetItemRequired)))))
    (CallFunction|DialogueAction)))

(fn ConstructionScript)

(fn DialogueCreate
  (Utilities|IsValid (Variables|Default|GetDialogueWidget)
    (:Is%20Valid
      _)
    (:Is%20Not%20Valid
      (bind _returnvalue (UserInterface|CreateWidget "/Game/MemoryYou_assets/Widgets/HUB_Dialogue.HUB_Dialogue_C"))
      (bind _output_get (Variables|Default|SetDialogueWidget _returnvalue))
      (UserInterface|Viewport|AddtoViewport _output_get 0)))
  (Variables|Default|SetMyMessage (Utilities|Array|MakeArray))
  (for _array_element (Variables|Default|GetMyDialogue)
    (bind _returnvalue_2 (Utilities|GetDataTableRow (Variables|Default|GetDialogueTable) _array_element)
      (:then
        (if (and (and (== (.MessageNo (Utilities|Struct|BreakDataTable_Dialogue_Struc _returnvalue_2)) (Variables|Default|GetMessageCurrent)) (Math|Boolean|Equal(Boolean) (.QuestComplete (Utilities|Struct|BreakDataTable_Dialogue_Struc _returnvalue_2)) (Variables|Default|GetQuestionComplete))) (Math|Boolean|Equal(Boolean) (.Again (Utilities|Struct|BreakDataTable_Dialogue_Struc _returnvalue_2)) (Variables|Default|GetAgain)))
          (Utilities|Array|Add (Variables|Default|GetMyMessage) (.Text (Utilities|Struct|BreakDataTable_Dialogue_Struc _returnvalue_2)))
          (Variables|Default|SetCurrentSpeak (.CharacterName (Utilities|Struct|BreakDataTable_Dialogue_Struc _returnvalue_2)))))))
  (CallFunction|DialogueShow))

(fn DialogueShow
  (bind _mymessage (Variables|Default|GetMyMessage))
  (bind _mymessage_2 (Variables|Default|GetMyMessage))
  (bind _returnvalue (Utilities|Array|Length _mymessage_2))
  (Variables|/Game/MemoryYou_assets/Widgets/HUB_Dialogue.HUB_Dialogue_C|SetText2 (Variables|Default|GetDialogueWidget) "")
  (Variables|/Game/MemoryYou_assets/Widgets/HUB_Dialogue.HUB_Dialogue_C|SetText1 (Variables|Default|GetDialogueWidget) "")
  (Variables|/Game/MemoryYou_assets/Widgets/HUB_Dialogue.HUB_Dialogue_C|SetText (Variables|Default|GetDialogueWidget) "")
  (Development|PrintString (Utilities|String|ToString(Integer) _returnvalue))
  (if (== _returnvalue 3)
    (Variables|/Game/MemoryYou_assets/Widgets/HUB_Dialogue.HUB_Dialogue_C|SetText2 (Variables|Default|GetDialogueWidget) (Utilities|Array|Get(acopy) _mymessage 2))
    (Variables|/Game/MemoryYou_assets/Widgets/HUB_Dialogue.HUB_Dialogue_C|SetText1 (Variables|Default|GetDialogueWidget) (Utilities|Array|Get(acopy) _mymessage 1) :!label _label)
    (Variables|/Game/MemoryYou_assets/Widgets/HUB_Dialogue.HUB_Dialogue_C|SetText (Variables|Default|GetDialogueWidget) (Utilities|Array|Get(acopy) _mymessage) :!label _label_2)
    (Variables|/Game/MemoryYou_assets/Widgets/HUB_Dialogue.HUB_Dialogue_C|SetEnum_Name (Variables|Default|GetDialogueWidget) (Variables|Default|GetCurrentSpeak))
    (elif (== _returnvalue 2)
      (goto _label)
      (elif (== _returnvalue 1)
        (goto _label_2)
        (else
          (Widget|RemovefromParent (Variables|Default|GetDialogueWidget))
          (Variables|Default|SetDialogueWidget 0)
          (Variables|Default|SetMessageCurrent 0)
          (if (not (Variables|Default|GetAgain))
            (Variables|Default|SetAgain true)
            (Actor|DestroyActor)
            (Actor|DestroyActor (Variables|Default|GetQuestionMarkReference))
            (Default|AddItem (Variables|Default|GetMainCharacterReference) (Variables|Default|GetItemName))))))))

(fn DialogueAction
  (Math|Integer|IncrementInt (Variables|Default|GetMessageCurrent)
    (:%20%20
      (CallFunction|DialogueCreate))))